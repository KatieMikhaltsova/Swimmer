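; BP_ParentSwimmer is a base Blueprint for swimmers that drift at a speed and direction set per level.
; BeginPlay looks up the current level name in a Struct to pick the speed.
; Each Tick adds a frame-time-scaled local X/Y offset from that level's StartMove vector.
; GetColorShip derives a color number from the Hat material's index in the Struct's material list.
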(event EventTick
  (params (DeltaSeconds :type Float%20%28single-precision%29))
  (bind _struct (Variables|Default|GetStruct))
  (bind (_levelname _spawnlocation _timerspawnships _levelspeed _levelamountships _levelamountcolorships _startmove) (Utilities|Struct|BreakBP_Str _struct))
  (Transformation|AddActorLocalOffset (Math|Vector|MakeVector (* (Utilities|Time|GetWorldDeltaSeconds) (Variables|Default|GetSpeed) (.X (Math|Vector|BreakVector (Utilities|Array|Get(acopy) _startmove (Utilities|Array|FindItem _levelname (stale EventBeginPlay _returnvalue)))))) (* (Utilities|Time|GetWorldDeltaSeconds) (Variables|Default|GetSpeed) (.Y (Math|Vector|BreakVector (Utilities|Array|Get(acopy) _startmove (Utilities|Array|FindItem _levelname (stale EventBeginPlay _returnvalue)))))) 0.0) false false))

(event EventBeginPlay
  (bind _struct (Variables|Default|GetStruct))
  (bind (_levelname _spawnlocation _timerspawnships _levelspeed _levelamountships _levelamountcolorships _startmove) (Utilities|Struct|BreakBP_Str _struct))
  (bind _returnvalue (Game|GetCurrentLevelName true))
  (Variables|Default|SetSpeed (Utilities|Array|Get(acopy) _levelspeed (Utilities|Array|FindItem _levelname _returnvalue))))

(fn ConstructionScript)

(fn GetColorShip
  (return (+ (Utilities|Array|FindItem (.Material (Utilities|Struct|BreakBP_Str (Variables|Default|GetStruct))) (Rendering|Material|GetMaterial (Variables|Default|GetHat) 0)) 1)))