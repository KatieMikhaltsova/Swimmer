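; Parent road piece that turns passing swimmers and, unless fixed, can be switched by touch with its linked ChangeRoad.
; A touch flips visibility and UseRotation on both pieces.
; On overlap, fixed or active pieces run a timeline applying incremental yaw up to 90 degrees times RotationShip, paced by swimmer speed and frame delta.
; Switchable pairs block touch during the turn; construction applies initial mesh visibility and shadow offset.
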(event OnComponentBeginOverlap(Box)
  (params (OverlappedComponent :type Primitive%20Component%20Object%20Reference) (OtherActor :type Actor%20Object%20Reference) (OtherComp :type Primitive%20Component%20Object%20Reference) (OtherBodyIndex :type Integer) (bFromSweep :type Boolean) (SweepResult :type Hit%20Result%20Structure%20%28by%20ref%29))
  (bind _asbp_parent_swimmer (Utilities|Casting|CastToBP_ParentSwimmer OtherActor))
  (Variables|Default|SetSwimmer _asbp_parent_swimmer)
  (if (Variables|Default|GetFix)
    (Variables|Default|SetPreviousCorner 0.0)
    (Components|Timeline|SetPlayRate (Variables|Default|GetSwimmerRotation) (* (Utilities|Time|GetWorldDeltaSeconds) (/ (Variables|/Game/Blueprints/Swimmer/BP_ParentSwimmer.BP_ParentSwimmer_C|GetSpeed (Variables|Default|GetSwimmer)) 5e+01) 1.2e+02))
    (bind _rotationswimmer (Timeline|SwimmerRotation PlayFromStart)
      (:Update
        (Transformation|AddActorLocalRotation (Variables|Default|GetSwimmer) (Math|Rotator|MakeRotator 0.0 0.0 (* (- (Math|Float|Lerp 0.0 9e+01 _rotationswimmer) (Variables|Default|GetPreviousCorner)) (Variables|Default|GetRotationShip))) false false)
        (Variables|Default|SetPreviousCorner (Math|Float|Lerp 0.0 9e+01 _rotationswimmer))))
    (elif (Variables|Default|GetUseRotation)
      (Variables|Default|SetBlockTouch true)
      (Variables|BP_ParentRoad_C|SetBlockTouch (Variables|Default|GetChangeRoad) true)
      (Variables|Default|SetPreviousCorner 0.0)
      (Components|Timeline|SetPlayRate (Variables|Default|GetSwimmerRotation_1) (* (Utilities|Time|GetWorldDeltaSeconds) (/ (Variables|/Game/Blueprints/Swimmer/BP_ParentSwimmer.BP_ParentSwimmer_C|GetSpeed (Variables|Default|GetSwimmer)) 5e+01) 1.2e+02))
      (bind _rotationswimmer_2 (Timeline|SwimmerRotation_1 PlayFromStart)
        (:Update
          (Transformation|AddActorLocalRotation (Variables|Default|GetSwimmer) (Math|Rotator|MakeRotator 0.0 0.0 (* (- (Math|Float|Lerp 0.0 9e+01 _rotationswimmer_2) (Variables|Default|GetPreviousCorner)) (Variables|Default|GetRotationShip))) false false)
          (Variables|Default|SetPreviousCorner (Math|Float|Lerp 0.0 9e+01 _rotationswimmer_2)))
        (:Finished
          (Variables|Default|SetBlockTouch false)
          (Variables|BP_ParentRoad_C|SetBlockTouch (Variables|Default|GetChangeRoad) false))))))

(event OnInputTouchBegin(Box)
  (params (FingerIndex :type ETouchIndex%20Enum :default "Touch1") (TouchedComponent :type Primitive%20Component%20Object%20Reference))
  ;[1 1 1] Road toggle
  (if (not (or (Variables|Default|GetFix) (Variables|Default|GetBlockTouch)))
    (Rendering|ToggleVisibility (Variables|Default|GetStaticMesh) true)
    (Rendering|ToggleVisibility (Variables|/Script/Engine.Actor|GetRootComponent (Variables|Default|GetChangeRoad)) true)
    (Variables|Default|SetUseRotation (not (Variables|Default|GetUseRotation)))
    (Variables|BP_ParentRoad_C|SetUseRotation (Variables|Default|GetChangeRoad) (not (Variables|BP_ParentRoad_C|GetUseRotation (Variables|Default|GetChangeRoad))))))

(fn ConstructionScript
  (Utilities|FlowControl|Sequence
    (:then_0
      (if (not (Variables|Default|GetVisibility))
        (Rendering|SetVisibility (Variables|Default|GetStaticMesh) false true)))
    (:then_1
      (Transformation|AddLocalOffset (Variables|Default|GetShadow) (Variables|Default|GetShadowOffset) false false))))