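; Level-manager pawn that spawns colored swimmers (called ships internally) and tallies how many reach their target.
; Once begun, Tick calls SpawnLoco, which uses per-level Struct data and a timer to space spawns up to the level's limit.
; Each swimmer gets a random swimsuit and a color differing from the previous two.
; When the spawn counter hits that limit, it saves a level-weighted score and opens the End level.
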(event Custom|SetAmountShipsSpawn
  (bind _struct (Variables|LevelData|GetStruct))
  (bind (_levelname _spawnlocation _timerspawnships _levelspeed _levelamountships _levelamountcolorships _startmove _arraycolorships _levelnumber _score) (Utilities|Struct|BreakBP_Str _struct))
  (bind _output_get (Variables|AmountShips|SetAmountShipsSpawn (+ (Variables|AmountShips|GetAmountShipsSpawn) 1)))
  (if (== _output_get (Utilities|Array|Get(acopy) (.LevelAmountShips (Utilities|Struct|BreakBP_Str (Variables|LevelData|GetStruct))) (Variables|LevelData|GetLevelIndex)))
    (Default|SaveResult (Variables|AmountShips|GetSaveGame) (* (Variables|AmountShips|GetAmountShipsInTarget) _score (Utilities|Array|Get(acopy) _levelnumber (Utilities|Array|FindItem _levelname (Variables|LevelData|GetLevelName)))))
    (Game|OpenLevel(byName) "End")))

(event Custom|SetAmountShipsInTarget
  (Variables|AmountShips|SetAmountShipsInTarget (+ (Variables|AmountShips|GetAmountShipsInTarget) 1)))

(event EventTick
  (params (DeltaSeconds :type Float%20%28single-precision%29))
  (if (Variables|Spawn|GetStart)
    (CallFunction|SpawnLoco)))

(event EventBegin
  (bind _struct (Variables|LevelData|GetStruct))
  (bind (_levelname _spawnlocation _timerspawnships) (Utilities|Struct|BreakBP_Str _struct))
  (Variables|Spawn|SetStart true)
  (Variables|Spawn|SetTimerSpawnShip (Utilities|Array|Get(acopy) _timerspawnships (Utilities|Array|FindItem _levelname (Variables|LevelData|GetLevelName)))))

(event EventBeginPlay
  (bind _returnvalue (SaveGame|CreateSaveGameObject "/Game/Blueprints/BP_SaveGame.BP_SaveGame_C"))
  (Variables|AmountShips|SetSaveGame _returnvalue)
  (bind _returnvalue_2 (Game|GetCurrentLevelName true))
  (Variables|LevelData|SetLevelName _returnvalue_2))

(fn ConstructionScript)

(fn SpawnLoco
  (bind _struct (Variables|LevelData|GetStruct))
  (bind (_levelname _spawnlocation _timerspawnships _levelspeed _levelamountships _levelamountcolorships _startmove _arraycolorships _levelnumber _score _material _spawnrotation) (Utilities|Struct|BreakBP_Str _struct))
  (Variables|LevelData|SetLevelIndex (Utilities|Array|FindItem _levelname (Variables|LevelData|GetLevelName)))
  (if (Variables|Spawn|GetCanSpawnShip)
    (bind _returnvalue (CallFunction|RandomIndex))
    (bind _returnvalue_2 (Game|SpawnActorfromClass "/Game/Blueprints/Swimmer/BP_ParentSwimmer.BP_ParentSwimmer_C" (Math|Transform|MakeTransform (Utilities|Array|Get(acopy) _spawnlocation (Variables|LevelData|GetLevelIndex))) "AlwaysSpawn" 0 0))
    (Transformation|SetActorRotation _returnvalue_2 (Utilities|Array|Get(acopy) _spawnrotation (Variables|LevelData|GetLevelIndex)))
    (bind _swimsuit (CallFunction|RandomSwimsuit))
    (Class|SkinnedMeshComponent|SetSkeletalMesh (Variables|/Game/Blueprints/Swimmer/BP_ParentSwimmer.BP_ParentSwimmer_C|GetClothes _returnvalue_2) _swimsuit true)
    (Rendering|Material|SetMaterial (Variables|/Game/Blueprints/Swimmer/BP_ParentSwimmer.BP_ParentSwimmer_C|GetHat _returnvalue_2) 0 (Utilities|Array|Get(acopy) (.Material (Utilities|Struct|BreakBP_Str (Variables|LevelData|GetStruct))) _returnvalue))
    (bind _output_get (Variables|AmountShips|SetAmountShips (+ 1 (Variables|AmountShips|GetAmountShips))))
    (if (>= _output_get (Utilities|Array|Get(acopy) _levelamountships (Variables|LevelData|GetLevelIndex)))
      (Variables|Spawn|SetCanSpawnShip false)
      (else
        (Variables|Spawn|SetCanSpawnShip false)
        (Utilities|Time|SetTimerbyFunctionName 0 "TimerSpawmLoco" (Variables|Spawn|GetTimerSpawnShip))))))

(fn TimerSpawmLoco
  (Variables|Spawn|SetCanSpawnShip true))

(fn SaveResult
  (bind _amountshipsintarget (Variables|AmountShips|GetAmountShipsInTarget))
  (bind _returnvalue (SaveGame|LoadGamefromSlot "1"))
  (bind _asbp_save_game (Utilities|Casting|CastToBP_SaveGame _returnvalue))
  (if (>= _amountshipsintarget (Variables|/Game/Blueprints/BP_SaveGame.BP_SaveGame_C|GetBestResult _asbp_save_game))
    (Variables|/Game/Blueprints/BP_SaveGame.BP_SaveGame_C|SetBestResult _asbp_save_game _amountshipsintarget)
    (SaveGame|SaveGametoSlot 0 "1")))

(fn RandomIndex
  (bind _struct (Variables|LevelData|GetStruct))
  (bind (_levelname _spawnlocation _timerspawnships _levelspeed _levelamountships _levelamountcolorships _startmove _arraycolorships) (Utilities|Struct|BreakBP_Str _struct))
  (Variables|ColorShips|SetArrayColorShips _arraycolorships)
  (Utilities|Array|Resize (Variables|ColorShips|GetArrayColorShips) (Utilities|Array|Get(acopy) _levelamountcolorships (Variables|LevelData|GetLevelIndex)))
  (Utilities|Array|RemoveItem (Variables|ColorShips|GetArrayColorShips) (Variables|ColorShips|GetLastColorShip))
  (Utilities|Array|RemoveItem (Variables|ColorShips|GetArrayColorShips) (Variables|ColorShips|GetLastButOneShip))
  (Variables|ColorShips|SetLastButOneShip (Variables|ColorShips|GetLastColorShip))
  (bind _output_get (Variables|ColorShips|SetLastColorShip (Utilities|Array|Get(acopy) (Variables|ColorShips|GetArrayColorShips) (Math|Random|RandomInteger (Utilities|Array|Length (Variables|ColorShips|GetArrayColorShips))))))
  (return _output_get))

(fn TouchInput
  (bind _returnvalue (Game|GetPlayerController 0))
  (bind (_locationx _locationy) (Class|PlayerController|GetInputTouchState _returnvalue "Touch1"))
  (return (Math|Vector2D|MakeVector2D _locationx _locationy)))

(fn RandomSwimsuit
  (return (Utilities|Select :Index (Math|Random|RandomInteger 2) :Option%200 "/Game/Animation/swimmer/shorts.shorts" :Option%201 "/Game/Animation/swimmer/closed.closed")))