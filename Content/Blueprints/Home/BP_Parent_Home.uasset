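; BP_Parent_Home is the base Blueprint for a color-coded home that receives ships.
; On construction and BeginPlay it shuffles all homes in the level and gives each cage and flag pair a material by index; construction also offsets shadow components.
; An overlapping ship's color is matched to the cage's material index, updating BP_Pawn counters and playing a success or error sound.
; Either way the ship is destroyed and AnimCage toggles, then toggles again on a timer.
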(event OnComponentBeginOverlap(Collision)
  (params (OverlappedComponent :type Primitive%20Component%20Object%20Reference) (OtherActor :type Actor%20Object%20Reference) (OtherComp :type Primitive%20Component%20Object%20Reference) (OtherBodyIndex :type Integer) (bFromSweep :type Boolean) (SweepResult :type Hit%20Result%20Structure%20%28by%20ref%29))
  (bind _color (Class|IntColorShip|GetColorShip(Message) OtherActor))
  (if (== _color (+ (Utilities|Array|FindItem (.Material (Utilities|Struct|BreakBP_Str (Variables|Default|GetStruct))) (Rendering|Material|GetMaterial (Variables|Default|GetCage) 0)) 1))
    (bind _asbp_pawn (Utilities|Casting|CastToBP_Pawn (Game|Player|GetPlayerPawn 0)))
    (Default|SetAmountShipsinTarget _asbp_pawn)
    (Default|SetAmountShipsSpawn _asbp_pawn)
    (Audio|PlaySound2D "/Game/Sounds/target.target" 0.3 1.0 0.0 0 0)
    (else
      (bind _asbp_pawn_2 (Utilities|Casting|CastToBP_Pawn (Game|Player|GetPlayerPawn 0)))
      (Default|SetAmountShipsSpawn _asbp_pawn_2)
      (Audio|PlaySound2D "/Game/Sounds/error.error" 0.3 1.0 0.0 0 0)))
  (Actor|DestroyActor OtherActor)
  (CallFunction|PlayAnimation)
  (Utilities|Time|SetTimerbyFunctionName 0 "PlayAnimation" 2.0))

(event EventBeginPlay
  (bind _outactors (Actor|GetAllActorsOfClass "BP_Parent_Home_C"))
  (Variables|Default|SetArrayHomeOnLevel _outactors)
  (Variables|Default|SetAmmountHomeOnLevel (Utilities|Array|Length (Variables|Default|GetArrayHomeOnLevel)))
  (Utilities|Array|Shuffle (Variables|Default|GetArrayHomeOnLevel))
  (for _index (range 0 (- (Variables|Default|GetAmmountHomeOnLevel) 1))
    (Rendering|Material|SetMaterial (Variables|BP_Parent_Home_C|GetFlag_l (Utilities|Array|Get(acopy) (Variables|Default|GetArrayHomeOnLevel) _index)) 0 (Utilities|Array|Get(acopy) (.Material (Utilities|Struct|BreakBP_Str (Variables|Default|GetStruct))) _index))))

(fn ConstructionScript
  (Utilities|FlowControl|Sequence
    (:then_0
      (bind _outactors (Actor|GetAllActorsOfClass "BP_Parent_Home_C"))
      (Variables|Default|SetArrayHomeOnLevel _outactors)
      (Variables|Default|SetAmmountHomeOnLevel (Utilities|Array|Length (Variables|Default|GetArrayHomeOnLevel)))
      (Utilities|Array|Shuffle (Variables|Default|GetArrayHomeOnLevel))
      (for _index (range 0 (- (Variables|Default|GetAmmountHomeOnLevel) 1))
        (Rendering|Material|SetMaterial (Variables|BP_Parent_Home_C|GetCage (Utilities|Array|Get(acopy) (Variables|Default|GetArrayHomeOnLevel) _index)) 0 (Utilities|Array|Get(acopy) (.Material (Utilities|Struct|BreakBP_Str (Variables|Default|GetStruct))) _index))))
    (:then_1
      (Transformation|AddLocalOffset (Variables|Default|GetCage_shadow) (Variables|Default|GetShadowOffset) false false))))

(fn PlayAnimation
  (Variables|Default|SetAnimCage (not (Variables|Default|GetAnimCage))))

(fn GetColorShip
  (return 0))