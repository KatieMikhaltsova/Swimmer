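; BP_SaveGame is a save game object that records the latest result and the best (highest) result achieved.
; Its SaveResult event loads the existing slot, or creates a new save object if none exists, to read the stored best.
; It sets its own BestResult to the higher value, then writes itself, rather than the loaded object, back to the slot.
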(event Custom|SaveResult
  (params (Result :type Integer))
  (Variables|Default|SetResult Result)
  (bind _returnvalue (SaveGame|DoesSaveGameExist "1"))
  (if _returnvalue
    (bind _returnvalue_2 (SaveGame|LoadGamefromSlot "1"))
    (Variables|Default|SetSave%20Game _returnvalue_2)
    (else
      (bind _returnvalue_3 (SaveGame|CreateSaveGameObject "BP_SaveGame_C"))
      (Variables|Default|SetSave%20Game _returnvalue_3)))
  (bind _asbp_save_game (Utilities|Casting|CastToBP_SaveGame (Variables|Default|GetSave%20Game)))
  (if (>= (Variables|Default|GetResult) (Variables|BP_SaveGame_C|GetBestResult _asbp_save_game))
    (Variables|Default|SetBestResult (Variables|Default|GetResult))
    (else
      (Variables|Default|SetBestResult (Variables|BP_SaveGame_C|GetBestResult _asbp_save_game))))
  (SaveGame|SaveGametoSlot self "1"))